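; BPC_DamageSystem is an actor component that manages health, healing and incoming damage.
; TakeDamage uses the CanBeDamaged macro to route each DamageInfo hit to block, damage or no damage, based on death, invincibility and blocking, with per-hit overrides.
; Results fire blocked (with parry flag), death or damage response calls, the last only when interruptible or forced.
; Heal clamps health to MaxHealth and is ignored once dead.
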(fn `Heal`
  (params (HealthValue :type "Float (double-precision)"))
  (returns (NewHealth :type "Float (double-precision)"))
  (if (not (`self.IsDead`))
    (bind _output_get (set `self.Health` (`KismetMathLibrary.FClamp` (+ HealthValue (`self.Health`)) 0.0 (`self.MaxHealth`))))
    (return _output_get)))

(fn `TakeDamage`
  (params (DamageInfo :type "/Game/BP/Interfaces/Damage/S_DamageInfo Structure"))
  (returns (WasDamaged :type Boolean))
  (bind (_amount _damagetype _damageresponse _candamageinvinciblity _canbeblocked _canbeparried _canforceinterrupt) (break `/Game/BP/Interfaces/Damage/S_DamageInfo` DamageInfo))
  (`self.CanBeDamaged` _candamageinvinciblity _canbeblocked
    (:`BlockDamage`
      ; Blocked Damage
      (`self.OnBlocked` _canbeparried)
      (return false))
    (:`DoDamage`
      ; Update health after reduction
      (bind _output_get (set `self.Health` (- (`self.Health`) _amount)))
      ; Is dead (health <= 0 after reduction)
      (if (<= _output_get 0.0)
        (set `self.IsDead` true)
        (`self.OnDeath`)
        (return true)
        (else
          ; If still alive after reduction, if interruptable then call damage response.
          (if (or (`self.IsInterruptible`) _canforceinterrupt)
            (`self.OnDamageResponse` _damageresponse)
            (return true)))))
    (:`NoDamage`
      (return false))))