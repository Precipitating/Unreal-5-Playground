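; BP_Enemy_Crossbow is a ranged enemy variant that spawns and holds a crossbow and fires it at its target.
; On BeginPlay it spawns BP_Weapon_Crossbow, attaches it to a right-hand socket and signals the equip.
; DefaultAttack passes montage, damage info and a spine-to-target trace line to the AttackComponent's CrossbowAttack.
; It also supplies movement speeds per state, ideal attack and defend ranges, and healing through its damage system component.
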(event `self.ReceiveBeginPlay`
  (`parent.ReceiveBeginPlay`)
  (`/Game/BP/Interfaces/AI/BPI_EnemyAI.EquipWeapon`))

(event `/Game/BP/Interfaces/AI/BPI_EnemyAI.EquipWeapon`
  (bind _returnvalue (`|SpawnActorFromClass` "/Game/BP/Weapons/BP_Weapon_Crossbow.BP_Weapon_Crossbow_C" (`self.GetTransform`) "Undefined" "MultiplyWithRoot" null null))
  (bind _output_get (set `self.WeaponActor` _returnvalue))
  (bind _returnvalue_2 (`self.K2_AttachToComponent` _output_get (`self.Mesh`) "hand_rSocket_crossbow" "SnapToTarget" "SnapToTarget" "SnapToTarget" true))
  (set `self.IsHoldingWeapon` _returnvalue_2)
  (`self.OnWeaponEquip`))

(event `DefaultAttack`
  (params (AttackTarget :type "Actor Object Reference"))
  (`/Game/BP/Components/AttackComponent.CrossbowAttack` (`self.AttackComponent`) (make `/Game/BP/Components/S_AttackInfo` AttackTarget "/Game/Animations/Attacks/Crossbow/FiringRifle_UE_Anim_Montage.FiringRifle_UE_Anim_Montage" (make `/Game/BP/Interfaces/Damage/S_DamageInfo` 20.0 "NewEnumerator3" "NewEnumerator0" false false false true)) (`SceneComponent.GetSocketLocation` (`self.Mesh`) "spine_03") (`self.K2_GetActorLocation` AttackTarget)))

(fn `GetIdealRange`
  (returns (AttackRadius :type "Float (double-precision)") (DefendRadius :type "Float (double-precision)"))
  (return 1000.0 600.0))

(fn `Heal`
  (params (HealValue :type "Float (double-precision)"))
  (returns (NewHealth :type "Float (double-precision)"))
  (bind _newhealth (`/Game/BP/Components/DamageSystemComponent.Heal` (`self.BPC_DamageSystem`) HealValue))
  (return _newhealth))

(fn `SetMaxSpeed`
  (params (Speed :type "/Game/BP/Interfaces/AI/E_MovementSpeed Enum" :default "NewEnumerator0"))
  (returns (NewSpeed :type "Float (double-precision)"))
  (bind _output_get (set `CharacterMovementComponent.MaxWalkSpeed` (select `/Game/BP/Interfaces/AI/E_MovementSpeed` Speed :`NewEnumerator1` 400.0 :`NewEnumerator2` 600.0 :!type "Float (single-precision)") (`self.CharacterMovement`)))
  (return _output_get))

(fn `UserConstructionScript`
  (`parent.UserConstructionScript`))